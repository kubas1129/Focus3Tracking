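; Debug actor that visualizes VR motion controller input for both hands with text renders and colored arrows.
; Button and touch presses show the key's interaction profile, identifier and component on that hand's text, and store the identifier.
; Tick uses that identifier to display the live trigger or grip axis value.
; Trackpad axes rotate each hand's arrow, tinted through dynamic material instances, to the input direction.
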(event Custom|ShowDebugKey
  (params (InKey :type Key%20Structure :default "None"))
  (bind (_interactionprofile _hand _motionsource _indentifier _component) (Class|HeadMountedDisplayFunctionLibrary|BreakKey InKey))
  (Rendering|Components|TextRender|SetText (Utilities|Select :Index _hand :Left (Variables|Default|GetTextRender_DebugKeyLeft) :Right (Variables|Default|GetTextRender_DebugKeyRight) :AnyHand 0 :Pad 0 :ExternalCamera 0 :Gun 0 :HMD 0 :Special_1 0 :Special_2 0 :Special_3 0 :Special_4 0 :Special_5 0 :Special_6 0 :Special_7 0 :Special_8 0 :Special_9 0 :Special_10 0 :Special_11 0) (Utilities|Text|ToText(String) (Utilities|String|Append _interactionprofile " 
" _indentifier " " _component)))
  (|SetBy-RefVar (Utilities|Select :Index _hand :Left (Variables|Default|GetLeftIdentifier) :Right (Variables|Default|GetRightdentifier) :AnyHand "" :Pad "" :ExternalCamera "" :Gun "" :HMD "" :Special_1 "" :Special_2 "" :Special_3 "" :Special_4 "" :Special_5 "" :Special_6 "" :Special_7 "" :Special_8 "" :Special_9 "" :Special_10 "" :Special_11 "") _indentifier))

(event Custom|ShowRightAxisValue
  (params (Value :type Float%20%28single-precision%29))
  (Rendering|Components|TextRender|SetText (Variables|Default|GetTextRender_DebugAxisRight) (Utilities|Text|ToText(Float) Value "HalfToEven" false true 1 324 3)))

(event Custom|ShowLeftAxisValue
  (params (Value :type Float%20%28single-precision%29))
  (Rendering|Components|TextRender|SetText (Variables|Default|GetTextRender_DebugAxisLeft) (Utilities|Text|ToText(Float) Value "HalfToEven" false true 1 324 3)))

(event EventBeginPlay
  (bind _rightarrow (Variables|Default|GetRightArrow))
  (bind _leftarrow (Variables|Default|GetLeftArrow))
  (Utilities|FlowControl|Sequence
    (:then_0
      (bind _returnvalue (Rendering|Material|CreateDynamicMaterialInstance _rightarrow 0 (Rendering|Material|GetMaterial _rightarrow 0) "None" :!class /Script/Engine.PrimitiveComponent))
      (bind _output_get (Variables|Default|SetRightMatInst _returnvalue))
      (Rendering|Material|SetVectorParameterValue _output_get "Color" (Variables|Default|GetRightColor) :!class /Script/Engine.MaterialInstanceDynamic))
    (:then_1
      (bind _returnvalue_2 (Rendering|Material|CreateDynamicMaterialInstance _leftarrow 0 (Rendering|Material|GetMaterial _leftarrow 0) "None" :!class /Script/Engine.PrimitiveComponent))
      (bind _output_get_2 (Variables|Default|SetLeftMatInst _returnvalue_2))
      (Rendering|Material|SetVectorParameterValue _output_get_2 "Color" (Variables|Default|GetLeftColor) :!class /Script/Engine.MaterialInstanceDynamic))))

(event EventTick
  (params (DeltaSeconds :type Float%20%28single-precision%29))
  (Utilities|FlowControl|Sequence
    (:then_0
      (switch string (Variables|Default|GetLeftIdentifier)
        (:Trigger
          (CallFunction|ShowLeftAxisValue (Input|AxisValues|GetMotionControllerTriggerAxisLeft)))
        (:Grip
          (CallFunction|ShowLeftAxisValue (Input|AxisValues|GetMotionControllerGripAxisLeft)))))
    (:then_1
      (switch string (Variables|Default|GetRightdentifier)
        (:Trigger
          (CallFunction|ShowRightAxisValue (Input|AxisValues|GetMotionControllerTriggerAxisRight)))
        (:Grip
          (CallFunction|ShowRightAxisValue (Input|AxisValues|GetMotionControllerGripAxisRight)))))))

(event Input|ActionEvents|InputActionMotionControllerTrackpadLeft
  (params (Key :type Key%20Structure :default "None"))
  (:Pressed
    (CallFunction|ShowDebugKey Key)))

(event Input|ActionEvents|InputActionMotionControllerTrackpadRight
  (params (Key :type Key%20Structure :default "None"))
  (:Pressed
    (CallFunction|ShowDebugKey Key)))

(event Input|ActionEvents|InputActionMotionControllerTriggerLeft
  (params (Key :type Key%20Structure :default "None"))
  (:Pressed
    (CallFunction|ShowDebugKey Key)))

(event Input|ActionEvents|InputActionMotionControllerTriggerRight
  (params (Key :type Key%20Structure :default "None"))
  (:Pressed
    (CallFunction|ShowDebugKey Key)))

(event Input|ActionEvents|InputActionMotionControllerGripLeft
  (params (Key :type Key%20Structure :default "None"))
  (:Pressed
    (CallFunction|ShowDebugKey Key)))

(event Input|ActionEvents|InputActionMotionControllerGripRight
  (params (Key :type Key%20Structure :default "None"))
  (:Pressed
    (CallFunction|ShowDebugKey Key)))

(event Input|ActionEvents|InputActionMotionControllerTrackpadTouchLeft
  (params (Key :type Key%20Structure :default "None"))
  (:Pressed
    (CallFunction|ShowDebugKey Key)))

(event Input|ActionEvents|InputActionMotionControllerTrackpadTouchRight
  (params (Key :type Key%20Structure :default "None"))
  (:Pressed
    (CallFunction|ShowDebugKey Key)))

(event Input|ActionEvents|InputActionMotionControllerButton_A
  (params (Key :type Key%20Structure :default "None"))
  (:Pressed
    (CallFunction|ShowDebugKey Key)))

(event Input|ActionEvents|InputActionMotionControllerButton_B
  (params (Key :type Key%20Structure :default "None"))
  (:Pressed
    (CallFunction|ShowDebugKey Key)))

(event Input|ActionEvents|InputActionMotionControllerButton_X
  (params (Key :type Key%20Structure :default "None"))
  (:Pressed
    (CallFunction|ShowDebugKey Key)))

(event Input|ActionEvents|InputActionMotionControllerButton_Y
  (params (Key :type Key%20Structure :default "None"))
  (:Pressed
    (CallFunction|ShowDebugKey Key)))

(event Input|ActionEvents|InputActionMotionControllerMenuLeft
  (params (Key :type Key%20Structure :default "None"))
  (:Pressed
    (CallFunction|ShowDebugKey Key)))

(event Input|ActionEvents|InputActionMotionControllerGripRight
  (params (Key :type Key%20Structure :default "None"))
  (:Pressed
    (CallFunction|ShowDebugKey Key)))

(event Input|ActionEvents|InputActionMotionControllerGripTouchLeft
  (params (Key :type Key%20Structure :default "None"))
  (:Pressed
    (CallFunction|ShowDebugKey Key)))

(event Input|ActionEvents|InputActionMotionControllerGripTouchRight
  (params (Key :type Key%20Structure :default "None"))
  (:Pressed
    (CallFunction|ShowDebugKey Key)))

(event Input|ActionEvents|InputActionMotionControllerTriggerTouchLeft
  (params (Key :type Key%20Structure :default "None"))
  (:Pressed
    (CallFunction|ShowDebugKey Key)))

(event Input|ActionEvents|InputActionMotionControllerTriggerTouchRight
  (params (Key :type Key%20Structure :default "None"))
  (:Pressed
    (CallFunction|ShowDebugKey Key)))

(event Input|AxisEvents|InputAxisMotionControllerTrackpadLeft_X
  (params (AxisValue :type Float%20%28single-precision%29))
  (Transformation|SetWorldRotation (Variables|Default|GetLeftArrow) (Math|Conversions|RotationFromXVector (Math|Vector|Normalize (Math|Vector|MakeVector (Input|AxisValues|GetMotionControllerTrackpadLeft_Y) (Input|AxisValues|GetMotionControllerTrackpadLeft_X) 0.0))) false false))

(event Input|AxisEvents|InputAxisMotionControllerTrackpadLeft_Y
  (params (AxisValue :type Float%20%28single-precision%29))
  (Transformation|SetWorldRotation (Variables|Default|GetLeftArrow) (Math|Conversions|RotationFromXVector (Math|Vector|Normalize (Math|Vector|MakeVector (Input|AxisValues|GetMotionControllerTrackpadLeft_Y) (Input|AxisValues|GetMotionControllerTrackpadLeft_X) 0.0))) false false))

(event Input|AxisEvents|InputAxisMotionControllerTrackpadRight_X
  (params (AxisValue :type Float%20%28single-precision%29))
  (Transformation|SetWorldRotation (Variables|Default|GetRightArrow) (Math|Conversions|RotationFromXVector (Math|Vector|Normalize (Math|Vector|MakeVector (Input|AxisValues|GetMotionControllerTrackpadRight_Y) (Input|AxisValues|GetMotionControllerTrackpadRight_X) 0.0))) false false))

(event Input|AxisEvents|InputAxisMotionControllerTrackpadRight_Y
  (params (AxisValue :type Float%20%28single-precision%29))
  (Transformation|SetWorldRotation (Variables|Default|GetRightArrow) (Math|Conversions|RotationFromXVector (Math|Vector|Normalize (Math|Vector|MakeVector (Input|AxisValues|GetMotionControllerTrackpadRight_Y) (Input|AxisValues|GetMotionControllerTrackpadRight_X) 0.0))) false false))

(fn ConstructionScript)