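; BP_SpawnBall is a physics ball actor that returns to its starting position after falling too far.
; BeginPlay stores the Sphere component's world location as the origin.
; Tick checks the Sphere's height and, below a fixed world Z threshold, moves it back to that origin.
; Physics simulation is switched off around the move and re-enabled afterwards.
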(event EventBeginPlay
  (Variables|Default|SetOriginLocation (Transformation|GetWorldLocation (Variables|Default|GetSphere))))

(event EventTick
  (params (DeltaSeconds :type Float%20%28single-precision%29))
  (bind _sphere (Variables|Default|GetSphere))
  (if (< (.z (Transformation|GetWorldLocation (Variables|Default|GetSphere))) -6e+02)
    (Physics|SetSimulatePhysics _sphere false)
    (Transformation|SetWorldLocation _sphere (Variables|Default|GetOriginLocation) false false)
    (Physics|SetSimulatePhysics _sphere true)))

(fn ConstructionScript)