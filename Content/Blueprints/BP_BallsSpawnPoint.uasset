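; BP_BallsSpawnPoint is a spawner actor that continuously drops BP_Ball actors into the level.
; BeginPlay gathers eight spawn location components into an array.
; Tick feeds a Delay that acts as a repeating timer, spawning a ball at a random location's world transform roughly every 0.7 seconds, regardless of collision.
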(event EventBeginPlay
  (Variables|Default|SetSpawn%20Locations (Utilities|Array|MakeArray (Variables|Default|GetSpawnLoc_1) (Variables|Default|GetSpawnLoc_2) (Variables|Default|GetSpawnLoc_3) (Variables|Default|GetSpawnLoc_4) (Variables|Default|GetSpawnLoc_5) (Variables|Default|GetSpawnLoc_6) (Variables|Default|GetSpawnLoc_7) (Variables|Default|GetSpawnLoc_8))))

(event EventTick
  (params (DeltaSeconds :type Float%20%28single-precision%29))
  (Utilities|FlowControl|Delay 0.7)
  (Game|SpawnActorfromClass "/Game/Blueprints/BP_Ball.BP_Ball_C" (Transformation|GetWorldTransform (.OutItem (Utilities|Array|Random (Variables|Default|GetSpawn%20Locations)))) "AlwaysSpawn" 0 0))

(fn ConstructionScript)