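; BP_Ball is a short-lived AR ball that turns green when it meets tracked real-world geometry, then destroys itself eight seconds after spawning.
; Each tick it runs three short AR line traces through the sphere along its local up, right and forward axes against tracked objects.
; Any hit sets the material's Color parameter to green, with no reset; matching debug-line drawing is left unconnected.
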(event EventBeginPlay
  (Utilities|FlowControl|Delay 8.0)
  (Actor|DestroyActor))

(event Collision|EventActorBeginOverlap
  (params (OtherActor :type Actor%20Object%20Reference)))

(event EventTick
  (params (DeltaSeconds :type Float%20%28single-precision%29))
  (bind _sphere (Variables|Default|GetSphere))
  (bind _returnvalue (Transformation|GetWorldTransform _sphere))
  (bind _returnvalue_2 (Math|Vector|GetRightVector (.rotation _returnvalue)))
  (bind _returnvalue_3 (Math|Vector|GetForwardVector (.rotation _returnvalue)))
  (bind _returnvalue_4 (Math|Vector|GetUpVector (.rotation _returnvalue)))
  (Utilities|FlowControl|Sequence
    (:then_0
      (bind _returnvalue_5 (Class|ARBlueprintLibrary|LineTraceTrackedObjects3D (+ (.location _returnvalue) (* _returnvalue_4 1e+01)) (+ (.location _returnvalue) (* _returnvalue_4 -1e+01)) true true false))
      (if (> (Utilities|Array|Length _returnvalue_5) 0)
        (Rendering|Material|SetVectorParameterValueonMaterials (Variables|Default|GetSphere) "Color" "0.000000,1.000000, 0" :!label _label)))
    (:then_1
      (bind _returnvalue_6 (Class|ARBlueprintLibrary|LineTraceTrackedObjects3D (+ (.location _returnvalue) (* _returnvalue_2 1e+01)) (+ (.location _returnvalue) (* _returnvalue_2 -1e+01)) true true false))
      (if (> (Utilities|Array|Length _returnvalue_6) 0)
        (goto _label)))
    (:then_2
      (bind _returnvalue_7 (Class|ARBlueprintLibrary|LineTraceTrackedObjects3D (+ (.location _returnvalue) (* _returnvalue_3 1e+01)) (+ (.location _returnvalue) (* _returnvalue_3 -1e+01)) true true false))
      (if (> (Utilities|Array|Length _returnvalue_7) 0)
        (goto _label)))))

(fn ConstructionScript)