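; VR/AR player Blueprint that lets both motion controllers shoot and probe tracked real-world geometry.
; BeginPlay sets floor tracking and caches whether scene understanding and facial tracking are enabled; Escape quits.
; With scene understanding on, grips spawn BP_Bullet, while fully pulled triggers line-trace tracked objects, storing hit transforms and drawing debug lines and spheres.
; Tick also draws a debug sphere at the right-hand grip position.
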(event EventBeginPlay
  (Class|HeadMountedDisplayFunctionLibrary|SetTrackingOrigin "Floor")
  (Utilities|FlowControl|Sequence
    (:then_0
      (Variables|Default|SetIsEnableSceneUnderstanding (Class|ViveOpenXRSceneUnderstandingFunctionLibrary|GetIsSceneUnderstandingEnabled)))
    (:then_1
      (Variables|Default|SetIsEnableFacialTracking (Class|ViveOpenXRFacialTrackingFunctionLibrary|GetIsFacialTrackingEnabled)))))

(event EventTick
  (params (DeltaSeconds :type Float%20%28single-precision%29))
  (bind _motioncontrollerdata (Class|HeadMountedDisplayFunctionLibrary|GetMotionControllerData 0 "Right"))
  (if (.bValid (Utilities|Struct|BreakXRMotionControllerData _motioncontrollerdata))
    (Rendering|Debug|DrawDebugSphere (.GripPosition (Utilities|Struct|BreakXRMotionControllerData _motioncontrollerdata)) 16.0 12 "(R=1.000000,G=1.000000,B=1.000000,A=1.000000)" 0.1 1.0)))

(event Input|ActionEvents|InputActionMotionControllerTriggerLeft
  (params (Key :type Key%20Structure :default "None"))
  ;[1 1 1] Left Motion Controller
)

(event Input|ActionEvents|InputActionMotionControllerTriggerRight
  (params (Key :type Key%20Structure :default "None"))
  ;[1 1 1] Right Motion Controller
)

(event Input|ActionEvents|InputActionMotionControllerGripLeft
  (params (Key :type Key%20Structure :default "None"))
  ;[1 1 1] Left Motion Controller
  (:Pressed
    (if (Variables|Default|GetIsEnableSceneUnderstanding)
      (Game|SpawnActorfromClass "/Game/Blueprints/BP_Bullet.BP_Bullet_C" (Transformation|GetWorldTransform (Variables|Default|GetMotionController_L)) "AlwaysSpawn" self 0)
      (Development|PrintString "Hello"))))

(event Input|ActionEvents|InputActionMotionControllerGripRight
  (params (Key :type Key%20Structure :default "None"))
  ;[1 1 1] Right Motion Controller
  (:Pressed
    (if (Variables|Default|GetIsEnableSceneUnderstanding)
      (Game|SpawnActorfromClass "/Game/Blueprints/BP_Bullet.BP_Bullet_C" (Transformation|GetWorldTransform (Variables|Default|GetMotionController_R)) "AlwaysSpawn" self 0))))

(event Input|AxisEvents|InputAxisMotionControllerTriggerAxisLeft
  (params (AxisValue :type Float%20%28single-precision%29))
  (bind _motioncontroller_l (Variables|Default|GetMotionController_L))
  (bind _motioncontroller_l_2 (Variables|Default|GetMotionController_L))
  (bind _returnvalue (Transformation|GetWorldTransform _motioncontroller_l_2))
  (bind _returnvalue_2 (Transformation|GetWorldTransform _motioncontroller_l))
  ;[1 1 1] Left Motion Controller
  (if (and (Variables|Default|GetIsEnableSceneUnderstanding) (== AxisValue 1.0))
    (bind _returnvalue_3 (Class|ARBlueprintLibrary|LineTraceTrackedObjects3D (.location _returnvalue_2) (+ (.location _returnvalue_2) (* (Math|Vector|GetForwardVector (.rotation _returnvalue_2)) 1e+04)) true true false))
    (if (> (Utilities|Array|Length _returnvalue_3) 0)
      (Rendering|Debug|DrawDebugSphere (.location (Class|ARTraceResultLibrary|GetLocalTransform (Utilities|Array|Get(acopy) _returnvalue_3))) 4.0 12 "(R=1.000000,G=0.000000,B=0.000000,A=1.000000)" 0.0 3.0)
      (Variables|Default|SetHitLoc_L (.location (Class|ARTraceResultLibrary|GetLocalTransform (Utilities|Array|Get(acopy) _returnvalue_3))))
      (Variables|Default|SetHitRot_L (.rotation (Class|ARTraceResultLibrary|GetLocalTransform (Utilities|Array|Get(acopy) _returnvalue_3))))
      (Rendering|Debug|DrawDebugLine (.location _returnvalue) (Variables|Default|GetHitLoc_L) "(R=1.000000,G=0.982247,B=0.000000,A=1.000000)" 0.0 1.0)
      (else
        (Rendering|Debug|DrawDebugLine (.location _returnvalue) (+ (.location _returnvalue) (* (Math|Vector|GetForwardVector (.rotation _returnvalue)) 1e+04)) "(R=1.000000,G=0.982247,B=0.000000,A=1.000000)" 0.0 1.0)))))

(event Input|AxisEvents|InputAxisMotionControllerTriggerAxisRight
  (params (AxisValue :type Float%20%28single-precision%29))
  (bind _motioncontroller_r (Variables|Default|GetMotionController_R))
  (bind _motioncontroller_r_2 (Variables|Default|GetMotionController_R))
  (bind _returnvalue (Transformation|GetWorldTransform _motioncontroller_r_2))
  (bind _returnvalue_2 (Transformation|GetWorldTransform _motioncontroller_r))
  ;[1 1 1] Right Motion Controller
  (if (and (Variables|Default|GetIsEnableSceneUnderstanding) (== AxisValue 1.0))
    (bind _returnvalue_3 (Class|ARBlueprintLibrary|LineTraceTrackedObjects3D (.location _returnvalue) (+ (.location _returnvalue) (* (Math|Vector|GetForwardVector (.rotation _returnvalue)) 1e+04)) true true false))
    (if (> (Utilities|Array|Length _returnvalue_3) 0)
      (Rendering|Debug|DrawDebugSphere (.location (Class|ARTraceResultLibrary|GetLocalTransform (Utilities|Array|Get(acopy) _returnvalue_3))) 4.0 12 "(R=1.000000,G=0.000000,B=0.000000,A=1.000000)" 0.0 3.0)
      (Variables|Default|SetHitLoc_R (.location (Class|ARTraceResultLibrary|GetLocalTransform (Utilities|Array|Get(acopy) _returnvalue_3))))
      (Variables|Default|SetHitRot_R (.rotation (Class|ARTraceResultLibrary|GetLocalTransform (Utilities|Array|Get(acopy) _returnvalue_3))))
      (Rendering|Debug|DrawDebugLine (.location _returnvalue_2) (Variables|Default|GetHitLoc_R) "(R=1.000000,G=0.982247,B=0.000000,A=1.000000)" 0.0 1.0)
      (else
        (Rendering|Debug|DrawDebugLine (.location _returnvalue_2) (+ (.location _returnvalue_2) (* (Math|Vector|GetForwardVector (.rotation _returnvalue_2)) 1e+04)) "(R=1.000000,G=0.982247,B=0.000000,A=1.000000)" 0.0 1.0)))))

(event Input|KeyboardEvents|Escape
  (params (Key :type Key%20Structure :default "None"))
  (:Pressed
    (Game|QuitGame 0 "Quit" false)))

(fn ConstructionScript)