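; Eye-tracked dart board actor that passes the gazed-at ring and pie segment to its material.
; On first valid gaze data, or when Z is pressed, it moves to its original offset from the camera and turns to face it.
; Each tick it line-traces along the gaze direction and, on a hit, feeds board axes, scale and bend/pie indices from helper functions into a dynamic material instance.
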(event EventTick
  (params (DeltaSeconds :type Float%20%28single-precision%29))
  (bind _returnvalue (Game|GetPlayerCameraManager 0))
  (bind _returnvalue_2 (Game|GetPlayerCameraManager 0))
  (bind _returnvalue_3 (Transformation|GetActorLocation))
  (bind _matinst (Variables|Default|GetMatInst))
  (bind _returnvalue_4 (Camera|GetCameraLocation _returnvalue))
  (bind _returnvalue_5 (Camera|GetCameraLocation _returnvalue_2))
  (bind _returnvalue_6 (Math|Rotator|FindLookatRotation _returnvalue_3 _returnvalue_4))
  (bind (_roll _pitch _yaw) (Math|Rotator|BreakRotator _returnvalue_6))
  (bind (_outgazedata _returnvalue_7) (Class|EyeTrackerFunctionLibrary|GetGazeData))
  (Variables|Default|SetOut%20Gaze%20Data _outgazedata)
  (Utilities|FlowControl|Sequence
    (:then_0
      (if (and _returnvalue_7 (not (Variables|Default|GetAlreadyMoveDart)))
        ;[1 1 1] Set dart board location and rotation
        (Utilities|FlowControl|Sequence
          (:then_0
            (Transformation|SetActorLocation (+ _returnvalue_4 (Variables|Default|GetOriginalLocation)) false false)
            (Transformation|SetActorRotation (Math|Rotator|MakeRotator _roll 0.0 (+ _yaw 1.8e+02))))
          (:then_1
            (Variables|Default|SetAlreadyMoveDart true)))))
    (:then_1
      ;[1 1 1] Use gaze date to line trace
      (if _returnvalue_7
        (bind (_outhit _returnvalue_8) (Collision|LineTraceByChannel _returnvalue_5 (+ _returnvalue_5 (* (Math|Vector|RotateVector (.gazedirection (Variables|Default|GetOut%20Gaze%20Data)) (Camera|GetCameraRotation _returnvalue_2)) 1e+03)) "TraceTypeQuery1" true (Utilities|Array|MakeArray _returnvalue_2) "ForDuration" false "(R=1.000000,G=0.000000,B=0.000000,A=1.000000)" "(R=0.000000,G=1.000000,B=0.000000,A=1.000000)" 0.2))
        (if _returnvalue_8
          (Variables|Default|SetFocusPos (.Location (Collision|BreakHitResult _outhit)))
          ;[1 1 1] Update dart board material
          (Rendering|Material|SetVectorParameterValue _matinst "MeshCenter" (Math|Conversions|ToLinearColor(Vector) (Transformation|GetActorLocation)) :!class /Script/Engine.MaterialInstanceDynamic)
          (Rendering|Material|SetVectorParameterValue _matinst "MeshForward" (Math|Conversions|ToLinearColor(Vector) (Transformation|GetActorForwardVector)) :!class /Script/Engine.MaterialInstanceDynamic)
          (Rendering|Material|SetVectorParameterValue _matinst "MeshRight" (Math|Conversions|ToLinearColor(Vector) (Transformation|GetActorRightVector)) :!class /Script/Engine.MaterialInstanceDynamic)
          (Rendering|Material|SetScalarParameterValue _matinst "BendIndex" (Math|Conversions|ToFloat(Integer) (Utilities|CalculateBendIndex)) :!class /Script/Engine.MaterialInstanceDynamic)
          (Rendering|Material|SetScalarParameterValue _matinst "PieIndex" (Math|Conversions|ToFloat(Integer) (Utilities|CalculatePieIndex)) :!class /Script/Engine.MaterialInstanceDynamic)
          (Rendering|Material|SetScalarParameterValue _matinst "Scale" (.y (Transformation|GetActorScale3D)) :!class /Script/Engine.MaterialInstanceDynamic))))))

(event EventBeginPlay
  (bind _dartboard (Variables|Default|GetDartBoard))
  (bind _returnvalue (Rendering|Material|CreateDynamicMaterialInstance _dartboard 0 (Rendering|Material|GetMaterial _dartboard 0) "None" :!class /Script/Engine.PrimitiveComponent))
  (bind _output_get (Variables|Default|SetMatInst _returnvalue))
  (Rendering|Material|SetScalarParameterValue _output_get "BendCount" (Math|Conversions|ToFloat(Integer) (Variables|BoardParameters|GetBendCount)) :!class /Script/Engine.MaterialInstanceDynamic)
  (Rendering|Material|SetScalarParameterValue _output_get "PieCount" (Math|Conversions|ToFloat(Integer) (Variables|BoardParameters|GetPieCount)) :!class /Script/Engine.MaterialInstanceDynamic)
  (Rendering|Material|SetScalarParameterValue _output_get "FrameWidth" (Math|Conversions|ToFloat(Integer) (Variables|BoardParameters|GetFrameWidth)) :!class /Script/Engine.MaterialInstanceDynamic)
  (Variables|Default|SetOriginalLocation (Transformation|GetActorLocation))
  (Input|EnableInput (Game|GetPlayerController 0)))

(event Input|KeyboardEvents|Z
  (params (Key :type Key%20Structure))
  (bind _returnvalue (Game|GetPlayerCameraManager 0))
  (bind _returnvalue_2 (Transformation|GetActorLocation))
  (bind _returnvalue_3 (Camera|GetCameraLocation _returnvalue))
  (bind _returnvalue_4 (Math|Rotator|FindLookatRotation _returnvalue_2 _returnvalue_3))
  (bind (_roll _pitch _yaw) (Math|Rotator|BreakRotator _returnvalue_4))
  (:Pressed
    ;[1 1 1] Set dart board location and rotation
    (Transformation|SetActorLocation (+ _returnvalue_3 (Variables|Default|GetOriginalLocation)) false false)
    (Transformation|SetActorRotation (Math|Rotator|MakeRotator _roll 0.0 (+ _yaw 1.8e+02)))))

(fn ConstructionScript)