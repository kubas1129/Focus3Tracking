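; Hand-tracking actor that visualizes both XR hands as debug rendering, static meshes or rigged hand actors, with SpaceBar cycling between modes.
; Tick reads motion controller data per hand and toggles visibility to suit the active mode.
; In static-mesh mode, RenderFinger moves collision-enabled joint meshes to keypoints.
; SetLinksTransform forms bones by centering, rotating and length-scaling link meshes between keypoint pairs.
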(event EventBeginPlay
  (CallFunction|SetRightHand)
  (CallFunction|SetLeftHand)
  (Variables|Default|SetHandKeypointCount (+ (Math|Conversions|ToInteger(Byte) (Variables|Default|GetHandKeyPoint_LittleTip)) 1))
  (Input|EnableInput (Game|GetPlayerController 0)))

(event EventTick
  (params (DeltaSeconds :type Float%20%28single-precision%29))
  (bind _lefthand (Variables|Default|GetLeftHand))
  (bind _rightlinks (Variables|Default|GetRightLinks))
  (bind _leftjoints (Variables|Default|GetLeftJoints))
  (bind _leftlinks (Variables|Default|GetLeftLinks))
  (bind _righthand (Variables|Default|GetRightHand))
  (bind _rightjoints (Variables|Default|GetRightJoints))
  (switch Utilities|FlowControl|Switch|SwitchonHandType (Variables|Default|GetHandType)
    (:NewEnumerator0
      (for _array_element (Variables|Default|GetRiggedHands)
        (Utilities|IsValid _array_element
          (:Is%20Valid
            (Rendering|SetActorHiddenInGame _array_element true))))
      (Rendering|SetVisibility (Variables|Default|GetRightHand) false true)
      (Utilities|FlowControl|Sequence
        (:then_0
          ;[1 1 1] Debug Right Hand
          (bind _motioncontrollerdata (Class|HeadMountedDisplayFunctionLibrary|GetMotionControllerData 0 "Right"))
          (Class|XRVisualizationFunctionLibrary|RenderMotionController _motioncontrollerdata true))
        (:then_1
          ;[1 1 1] Debug Left Hand
          (bind _motioncontrollerdata_2 (Class|HeadMountedDisplayFunctionLibrary|GetMotionControllerData 0 "Left"))
          (Class|XRVisualizationFunctionLibrary|RenderMotionController _motioncontrollerdata_2 false))))
    (:NewEnumerator1
      (for _array_element_2 (Variables|Default|GetRiggedHands)
        (Utilities|IsValid _array_element_2
          (:Is%20Valid
            (Rendering|SetActorHiddenInGame _array_element_2 true))))
      (Utilities|FlowControl|Sequence
        (:then_0
          ;[1 1 1] StaticMesh Right Hand
          (bind _motioncontrollerdata_3 (Class|HeadMountedDisplayFunctionLibrary|GetMotionControllerData 0 "Right"))
          (CallFunction|SetLinksTransform 0 (Utilities|Array|Get(acopy) (.HandKeyPositions (Utilities|Struct|BreakXRMotionControllerData _motioncontrollerdata_3))) (Utilities|Array|Get(acopy) (.HandKeyPositions (Utilities|Struct|BreakXRMotionControllerData _motioncontrollerdata_3)) 1) (Variables|Default|GetRightLinks))
          (CallFunction|RenderFinger _motioncontrollerdata_3 "ThumbMetacarpal" "ThumbTip" _righthand _rightlinks _rightjoints)
          (CallFunction|RenderFinger _motioncontrollerdata_3 "IndexMetacarpal" "IndexTip" _righthand _rightlinks _rightjoints)
          (CallFunction|RenderFinger _motioncontrollerdata_3 "MiddleMetacarpal" "MiddleTip" _righthand _rightlinks _rightjoints)
          (CallFunction|RenderFinger _motioncontrollerdata_3 "RingMetacarpal" "RingTip" _righthand _rightlinks _rightjoints)
          (CallFunction|RenderFinger _motioncontrollerdata_3 "LittleMetacarpal" "LittleTip" _righthand _rightlinks _rightjoints))
        (:then_1
          ;[1 1 1] StaticMesh Left Hand
          (bind _motioncontrollerdata_4 (Class|HeadMountedDisplayFunctionLibrary|GetMotionControllerData 0 "Left"))
          (CallFunction|SetLinksTransform 0 (Utilities|Array|Get(acopy) (.HandKeyPositions (Utilities|Struct|BreakXRMotionControllerData _motioncontrollerdata_4))) (Utilities|Array|Get(acopy) (.HandKeyPositions (Utilities|Struct|BreakXRMotionControllerData _motioncontrollerdata_4)) 1) (Variables|Default|GetLeftLinks))
          (CallFunction|RenderFinger _motioncontrollerdata_4 "ThumbMetacarpal" "ThumbTip" _lefthand _leftlinks _leftjoints)
          (CallFunction|RenderFinger _motioncontrollerdata_4 "IndexMetacarpal" "IndexTip" _lefthand _leftlinks _leftjoints)
          (CallFunction|RenderFinger _motioncontrollerdata_4 "MiddleMetacarpal" "MiddleTip" _lefthand _leftlinks _leftjoints)
          (CallFunction|RenderFinger _motioncontrollerdata_4 "RingMetacarpal" "RingTip" _lefthand _leftlinks _leftjoints)
          (CallFunction|RenderFinger _motioncontrollerdata_4 "LittleMetacarpal" "LittleTip" _lefthand _leftlinks _leftjoints))))
    (:NewEnumerator2
      (Rendering|SetVisibility (Variables|Default|GetRightHand) false true)
      (for _array_element_3 (Variables|Default|GetRiggedHands)
        (Utilities|IsValid _array_element_3
          (:Is%20Valid
            (Rendering|SetActorHiddenInGame _array_element_3 false)))))))

(event EventEndPlay
  (params (EndPlayReason :type EEndPlayReason%20Enum :default "Destroyed"))
  (Utilities|Array|Clear (Variables|Default|GetRightJoints))
  (Utilities|Array|Clear (Variables|Default|GetRightLinks))
  (Utilities|Array|Clear (Variables|Default|GetLeftJoints))
  (Utilities|Array|Clear (Variables|Default|GetLeftLinks)))

(event Input|KeyboardEvents|SpaceBar
  (params (Key :type Key%20Structure :default "None"))
  (:Pressed
    (CallFunction|SwitchHand)))

(fn ConstructionScript)

(fn SetRightHand
  (bind _rj23 (Variables|Default|GetRJ23))
  (bind _rj24 (Variables|Default|GetRJ24))
  (bind _rj22 (Variables|Default|GetRJ22))
  (bind _rj11 (Variables|Default|GetRJ11))
  (bind _rj2 (Variables|Default|GetRJ2))
  (bind _rj3 (Variables|Default|GetRJ3))
  (bind _rj4 (Variables|Default|GetRJ4))
  (bind _rj5 (Variables|Default|GetRJ5))
  (bind _rj6 (Variables|Default|GetRJ6))
  (bind _rj7 (Variables|Default|GetRJ7))
  (bind _rj8 (Variables|Default|GetRJ8))
  (bind _rj9 (Variables|Default|GetRJ9))
  (bind _rj10 (Variables|Default|GetRJ10))
  (bind _rj1 (Variables|Default|GetRJ1))
  (bind _rj12 (Variables|Default|GetRJ12))
  (bind _rj13 (Variables|Default|GetRJ13))
  (bind _rj14 (Variables|Default|GetRJ14))
  (bind _rj15 (Variables|Default|GetRJ15))
  (bind _rj16 (Variables|Default|GetRJ16))
  (bind _rj17 (Variables|Default|GetRJ17))
  (bind _rj18 (Variables|Default|GetRJ18))
  (bind _rj19 (Variables|Default|GetRJ19))
  (bind _rj20 (Variables|Default|GetRJ20))
  (bind _rj21 (Variables|Default|GetRJ21))
  (bind _rl13 (Variables|Default|GetRL13))
  (bind _rl2 (Variables|Default|GetRL2))
  (bind _rl3 (Variables|Default|GetRL3))
  (bind _rl4 (Variables|Default|GetRL4))
  (bind _rl5 (Variables|Default|GetRL5))
  (bind _rl6 (Variables|Default|GetRL6))
  (bind _rl7 (Variables|Default|GetRL7))
  (bind _rl8 (Variables|Default|GetRL8))
  (bind _rl9 (Variables|Default|GetRL9))
  (bind _rl10 (Variables|Default|GetRL10))
  (bind _rl11 (Variables|Default|GetRL11))
  (bind _rl12 (Variables|Default|GetRL12))
  (bind _rl1 (Variables|Default|GetRL1))
  (bind _rl14 (Variables|Default|GetRL14))
  (bind _rl15 (Variables|Default|GetRL15))
  (bind _rl16 (Variables|Default|GetRL16))
  (bind _rl17 (Variables|Default|GetRL17))
  (bind _rl18 (Variables|Default|GetRL18))
  (bind _rl19 (Variables|Default|GetRL19))
  (bind _rl20 (Variables|Default|GetRL20))
  (bind _rl21 (Variables|Default|GetRL21))
  (bind _rl22 (Variables|Default|GetRL22))
  (bind _rl23 (Variables|Default|GetRL23))
  (bind _rl24 (Variables|Default|GetRL24))
  (bind _rj26 (Variables|Default|GetRJ26))
  (bind _rj25 (Variables|Default|GetRJ25))
  (bind _rl25 (Variables|Default|GetRL25))
  (bind _array (Utilities|Array|MakeArray _rj1 _rj2 _rj3 _rj4 _rj5 _rj6 _rj7 _rj8 _rj9 _rj10 _rj11 _rj12 _rj13 _rj14 _rj15 _rj16 _rj17 _rj18 _rj19 _rj20 _rj21 _rj22 _rj23 _rj24 _rj25 _rj26))
  (bind _array_2 (Utilities|Array|MakeArray _rl1 _rl2 _rl3 _rl4 _rl5 _rl6 _rl7 _rl8 _rl9 _rl10 _rl11 _rl12 _rl13 _rl14 _rl15 _rl16 _rl17 _rl18 _rl19 _rl20 _rl21 _rl22 _rl23 _rl24 _rl25))
  (Utilities|Array|AppendArray (Variables|Default|GetRightJoints) _array)
  (for _array_element _array
    (Collision|SetCollisionEnabled _array_element "QueryAndPhysics"))
  (Utilities|Array|AppendArray (Variables|Default|GetRightLinks) _array_2)
  (for _array_element_2 _array_2
    (Collision|SetCollisionEnabled _array_element_2 "QueryAndPhysics"))
  (return))

(fn RenderFinger
  (params (XRControllerData :type XR%20Motion%20Controller%20Data%20Structure) (FingerStart :type EHandKeypoint%20Enum :default "Palm") (FingerEnd :type EHandKeypoint%20Enum :default "Palm") (Hand :type Scene%20Component%20Object%20Reference) (Links :type Array%20of%20Static%20Mesh%20Component%20Object%20References) (Joints :type Array%20of%20Static%20Mesh%20Component%20Object%20References))
  (bind (_bvalid _devicename _applicationinstanceid _devicevisualtype _handindex _trackingstatus _gripposition _griprotation _aimposition _aimrotation _handkeypositions _handkeyrotations _handkeyradii) (Utilities|Struct|BreakXRMotionControllerData XRControllerData))
  (bind _handkeypointcount (Variables|Default|GetHandKeypointCount))
  (LocalVariables|SetHandKeyRotations _handkeyrotations)
  (LocalVariables|SetHandKeyPositions _handkeypositions)
  (LocalVariables|SetHandKeyRadii _handkeyradii)
  (Rendering|SetVisibility Hand _bvalid true)
  (if (and (== (Utilities|Array|Length (LocalVariables|GetHandKeyPositions)) _handkeypointcount) (== _handkeypointcount (Utilities|Array|Length (LocalVariables|GetHandKeyRadii))))
    (CallFunction|SetLinksTransform (- (Class|HandKeypointConversion|ToInt32(HandKeypoint) FingerStart) 1) (Utilities|Array|Get(acopy) (LocalVariables|GetHandKeyPositions) 1) (Utilities|Array|Get(acopy) (LocalVariables|GetHandKeyPositions) (Class|HandKeypointConversion|ToInt32(HandKeypoint) FingerStart)) Links)
    (for _index (range (Class|HandKeypointConversion|ToInt32(HandKeypoint) FingerStart) (- (Class|HandKeypointConversion|ToInt32(HandKeypoint) FingerEnd) 1))
      (CallFunction|SetLinksTransform _index (Utilities|Array|Get(acopy) (LocalVariables|GetHandKeyPositions) _index) (Utilities|Array|Get(acopy) (LocalVariables|GetHandKeyPositions) (+ _index 1)) Links))
    (for (_array_element _array_index) Joints
      (Transformation|SetWorldLocation _array_element (Utilities|Array|Get(acopy) (LocalVariables|GetHandKeyPositions) _array_index) false false))))

(fn SetLinksTransform
  (params (LinkID :type Integer) (FirstPos :type Vector) (SecondPos :type Vector) (Links :type Array%20of%20Static%20Mesh%20Component%20Object%20References))
  (bind _returnvalue (- SecondPos FirstPos))
  (Transformation|SetWorldTransform (Utilities|Array|Get(acopy) Links LinkID) (Math|Transform|MakeTransform (/ (+ SecondPos FirstPos) 2.0) (Math|Rotator|MakeRotfromZX _returnvalue (Class|KismetMathLibrary|VectorForward)) (Math|Vector|MakeVector 0.01 0.01 (* (Math|Vector|VectorLength _returnvalue) 0.01))) false false))

(fn SetLeftHand
  (bind _lj22 (Variables|Default|GetLJ22))
  (bind _ll25 (Variables|Default|GetLL25))
  (bind _lj11 (Variables|Default|GetLJ11))
  (bind _lj2 (Variables|Default|GetLJ2))
  (bind _lj3 (Variables|Default|GetLJ3))
  (bind _lj4 (Variables|Default|GetLJ4))
  (bind _lj5 (Variables|Default|GetLJ5))
  (bind _lj6 (Variables|Default|GetLJ6))
  (bind _lj7 (Variables|Default|GetLJ7))
  (bind _lj8 (Variables|Default|GetLJ8))
  (bind _lj9 (Variables|Default|GetLJ9))
  (bind _lj10 (Variables|Default|GetLJ10))
  (bind _lj1 (Variables|Default|GetLJ1))
  (bind _lj12 (Variables|Default|GetLJ12))
  (bind _lj13 (Variables|Default|GetLJ13))
  (bind _lj14 (Variables|Default|GetLJ14))
  (bind _lj15 (Variables|Default|GetLJ15))
  (bind _lj16 (Variables|Default|GetLJ16))
  (bind _lj17 (Variables|Default|GetLJ17))
  (bind _lj18 (Variables|Default|GetLJ18))
  (bind _lj19 (Variables|Default|GetLJ19))
  (bind _lj20 (Variables|Default|GetLJ20))
  (bind _lj21 (Variables|Default|GetLJ21))
  (bind _ll13 (Variables|Default|GetLL13))
  (bind _ll2 (Variables|Default|GetLL2))
  (bind _ll3 (Variables|Default|GetLL3))
  (bind _ll4 (Variables|Default|GetLL4))
  (bind _ll5 (Variables|Default|GetLL5))
  (bind _ll6 (Variables|Default|GetLL6))
  (bind _ll7 (Variables|Default|GetLL7))
  (bind _ll8 (Variables|Default|GetLL8))
  (bind _ll9 (Variables|Default|GetLL9))
  (bind _ll10 (Variables|Default|GetLL10))
  (bind _ll11 (Variables|Default|GetLL11))
  (bind _ll12 (Variables|Default|GetLL12))
  (bind _ll1 (Variables|Default|GetLL1))
  (bind _ll14 (Variables|Default|GetLL14))
  (bind _ll15 (Variables|Default|GetLL15))
  (bind _ll16 (Variables|Default|GetLL16))
  (bind _ll17 (Variables|Default|GetLL17))
  (bind _ll18 (Variables|Default|GetLL18))
  (bind _ll19 (Variables|Default|GetLL19))
  (bind _ll20 (Variables|Default|GetLL20))
  (bind _ll21 (Variables|Default|GetLL21))
  (bind _ll22 (Variables|Default|GetLL22))
  (bind _ll23 (Variables|Default|GetLL23))
  (bind _ll24 (Variables|Default|GetLL24))
  (bind _lj23 (Variables|Default|GetLJ23))
  (bind _lj24 (Variables|Default|GetLJ24))
  (bind _lj25 (Variables|Default|GetLJ25))
  (bind _lj26 (Variables|Default|GetLJ26))
  (bind _array (Utilities|Array|MakeArray _lj1 _lj2 _lj3 _lj4 _lj5 _lj6 _lj7 _lj8 _lj9 _lj10 _lj11 _lj12 _lj13 _lj14 _lj15 _lj16 _lj17 _lj18 _lj19 _lj20 _lj21 _lj22 _lj23 _lj24 _lj25 _lj26))
  (bind _array_2 (Utilities|Array|MakeArray _ll1 _ll2 _ll3 _ll4 _ll5 _ll6 _ll7 _ll8 _ll9 _ll10 _ll11 _ll12 _ll13 _ll14 _ll15 _ll16 _ll17 _ll18 _ll19 _ll20 _ll21 _ll22 _ll23 _ll24 _ll25))
  (Utilities|Array|AppendArray (Variables|Default|GetLeftJoints) _array)
  (for _array_element _array
    (Collision|SetCollisionEnabled _array_element "QueryAndPhysics"))
  (Utilities|Array|AppendArray (Variables|Default|GetLeftLinks) _array_2)
  (for _array_element_2 _array_2
    (Collision|SetCollisionEnabled _array_element_2 "QueryAndPhysics"))
  (return))

(fn SwitchHand
  (if (Utilities|Enum|Equal(Enum) (Variables|Default|GetHandType) "NewEnumerator0")
    (Variables|Default|SetHandType "NewEnumerator1")
    (elif (Utilities|Enum|Equal(Enum) (Variables|Default|GetHandType) "NewEnumerator1")
      (Variables|Default|SetHandType "NewEnumerator2")
      (elif (Utilities|Enum|Equal(Enum) (Variables|Default|GetHandType) "NewEnumerator2")
        (Variables|Default|SetHandType "NewEnumerator0")))))