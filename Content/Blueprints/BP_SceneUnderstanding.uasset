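; Actor that runs ViveOpenXR Scene Understanding spatial mapping and toggles the scanned meshes between visible and occlusion rendering.
; BeginPlay sets compute bounds from CubeBound and starts AR capture, which retries on failure and auto-stops on a timer.
; ARTrackableNotify maintains the mesh list, and Tick reapplies the current mode by swapping material, main pass and custom depth.
; Controller and keyboard input flip visibility, with debug keys to start or stop mapping.
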(event OnAddTrackedGeometry(ARTrackableNotify)
  (params (TrackedGeometry :type AR%20Tracked%20Geometry%20Object%20Reference))
  (if (Variables|Default|GetIsEnableSceneUnderstanding)
    (Utilities|Array|AddUnique (Variables|Default|GetspatialMeshes) TrackedGeometry)))

(event OnRemoveTrackedGeometry(ARTrackableNotify)
  (params (TrackedGeometry :type AR%20Tracked%20Geometry%20Object%20Reference))
  (if (Variables|Default|GetIsEnableSceneUnderstanding)
    (Utilities|Array|RemoveItem (Variables|Default|GetspatialMeshes) TrackedGeometry)))

(event EventBeginPlay
  (bind _cube_bound (Variables|Default|GetCube_bound))
  ;[1 1 1] Initial
  (bind _output_get (Variables|Default|SetIsEnableSceneUnderstanding (Class|ViveOpenXRSceneUnderstandingFunctionLibrary|GetIsSceneUnderstandingEnabled)))
  (if _output_get
    (Input|EnableInput (Game|GetPlayerController 0))
    (Class|ViveOpenXRSceneUnderstandingFunctionLibrary|SetSceneComputeOrientedBoxBound (Transformation|GetWorldRotation _cube_bound) (Transformation|GetWorldLocation _cube_bound) (Transformation|GetWorldScale _cube_bound))
    (Class|ViveOpenXRSceneUnderstandingFunctionLibrary|SetSceneComputeConsistency "SnapshotIncompleteFast")
    (Class|ViveOpenXRSceneUnderstandingFunctionLibrary|SetMeshComputeLod "Medium")
    (CallFunction|StartSpatialMapping)
    (else
      (Development|PrintString "[Scene Understanding] Please enable Scene Understanding in Project Setting > Plugins > ViveOpenXR." true true "(R=1.000000,G=0.007701,B=0.000000,A=1.000000)" 6e+01))))

(event EventTick
  (params (DeltaSeconds :type Float%20%28single-precision%29))
  (if (and (Variables|Default|GetIsUpdateCompleted) (Variables|Default|GetIsEnableSceneUnderstanding))
    (if (Variables|Default|GetshowSpatialMapping)
      (Variables|Default|SetIsUpdateCompleted false)
      (for _array_element (Variables|Default|GetspatialMeshes)
        (CallFunction|ShowSpatialMeshes _array_element))
      (Variables|Default|SetIsUpdateCompleted true)
      (else
        (Variables|Default|SetIsUpdateCompleted false)
        (for _array_element_2 (Variables|Default|GetspatialMeshes)
          (CallFunction|HideSpatialMeshes _array_element_2))
        (Variables|Default|SetIsUpdateCompleted true)))))

(event EventEndPlay
  (params (EndPlayReason :type EEndPlayReason%20Enum :default "Destroyed"))
  ;[1 1 1] End Play
  (if (Variables|Default|GetIsEnableSceneUnderstanding)
    (CallFunction|StopSpatialMapping)
    (Class|ViveOpenXRSceneUnderstandingFunctionLibrary|ClearSceneComputeBounds "OrientedBox")
    (Utilities|Array|Clear (Variables|Default|GetspatialMeshes))))

(event Input|ActionEvents|InputActionMotionControllerTrackpadLeft
  (params (Key :type Key%20Structure :default "None"))
  (bind _spatialmeshes (Variables|Default|GetspatialMeshes))
  ;[1 1 1] Show / Hide Spatial Mapping
  (:Pressed
    (if (Variables|Default|GetIsEnableSceneUnderstanding)
      (Utilities|FlowControl|FlipFlop
        (:A
          (Variables|Default|SetshowSpatialMapping false)
          (for _array_element _spatialmeshes
            (CallFunction|HideSpatialMeshes _array_element))
          (Development|PrintString "Hide Mesh"))
        (:B
          (Variables|Default|SetshowSpatialMapping true)
          (for _array_element_2 _spatialmeshes
            (CallFunction|ShowSpatialMeshes _array_element_2))
          (Development|PrintString "Show Mesh"))))))

(event Input|ActionEvents|InputActionMotionControllerTrackpadRight
  (params (Key :type Key%20Structure :default "None"))
  (bind _spatialmeshes (Variables|Default|GetspatialMeshes))
  ;[1 1 1] Show / Hide Spatial Mapping
  (:Pressed
    (if (Variables|Default|GetIsEnableSceneUnderstanding)
      (Utilities|FlowControl|FlipFlop
        (:A
          (Variables|Default|SetshowSpatialMapping false)
          (for _array_element _spatialmeshes
            (CallFunction|HideSpatialMeshes _array_element))
          (Development|PrintString "Hide Mesh"))
        (:B
          (Variables|Default|SetshowSpatialMapping true)
          (for _array_element_2 _spatialmeshes
            (CallFunction|ShowSpatialMeshes _array_element_2))
          (Development|PrintString "Show Mesh"))))))

(event Input|ActionEvents|InputActionMotionControllerButton_A
  (params (Key :type Key%20Structure :default "None"))
  (bind _spatialmeshes (Variables|Default|GetspatialMeshes))
  ;[1 1 1] Show / Hide Spatial Mapping
  (:Pressed
    (if (Variables|Default|GetIsEnableSceneUnderstanding)
      (Utilities|FlowControl|FlipFlop
        (:A
          (Variables|Default|SetshowSpatialMapping false)
          (for _array_element _spatialmeshes
            (CallFunction|HideSpatialMeshes _array_element))
          (Development|PrintString "Hide Mesh"))
        (:B
          (Variables|Default|SetshowSpatialMapping true)
          (for _array_element_2 _spatialmeshes
            (CallFunction|ShowSpatialMeshes _array_element_2))
          (Development|PrintString "Show Mesh"))))))

(event Input|ActionEvents|InputActionMotionControllerButton_X
  (params (Key :type Key%20Structure :default "None"))
  (bind _spatialmeshes (Variables|Default|GetspatialMeshes))
  ;[1 1 1] Show / Hide Spatial Mapping
  (:Pressed
    (if (Variables|Default|GetIsEnableSceneUnderstanding)
      (Utilities|FlowControl|FlipFlop
        (:A
          (Variables|Default|SetshowSpatialMapping false)
          (for _array_element _spatialmeshes
            (CallFunction|HideSpatialMeshes _array_element))
          (Development|PrintString "Hide Mesh"))
        (:B
          (Variables|Default|SetshowSpatialMapping true)
          (for _array_element_2 _spatialmeshes
            (CallFunction|ShowSpatialMeshes _array_element_2))
          (Development|PrintString "Show Mesh"))))))

(event Input|KeyboardEvents|SpaceBar
  (params (Key :type Key%20Structure :default "None"))
  (bind _spatialmeshes (Variables|Default|GetspatialMeshes))
  ;[1 1 1] Show / Hide Spatial Mapping
  (:Pressed
    (if (Variables|Default|GetIsEnableSceneUnderstanding)
      (Utilities|FlowControl|FlipFlop
        (:A
          (Variables|Default|SetshowSpatialMapping false)
          (for _array_element _spatialmeshes
            (CallFunction|HideSpatialMeshes _array_element))
          (Development|PrintString "Hide Mesh"))
        (:B
          (Variables|Default|SetshowSpatialMapping true)
          (for _array_element_2 _spatialmeshes
            (CallFunction|ShowSpatialMeshes _array_element_2))
          (Development|PrintString "Show Mesh"))))))

(event Input|KeyboardEvents|A
  (params (Key :type Key%20Structure :default "None"))
  ;[1 1 1] start spatial mapping
  (:Pressed
    (if (Variables|Default|GetIsEnableSceneUnderstanding)
      (CallFunction|StartSpatialMapping))))

(event Input|KeyboardEvents|S
  (params (Key :type Key%20Structure :default "None"))
  ;[1 1 1] stop spatial mapping
  (:Pressed
    (if (Variables|Default|GetIsEnableSceneUnderstanding)
      (CallFunction|StopSpatialMapping))))

(fn ConstructionScript)

(fn ShowSpatialMeshes
  (params (TrackedGeometry :type AR%20Tracked%20Geometry%20Object%20Reference))
  (bind _returnvalue (Class|ARTrackedGeometry|GetUnderlyingMesh TrackedGeometry))
  (if (Utilities|IsValid _returnvalue)
    (Rendering|SetRenderCustomDepth _returnvalue false)
    (Class|PrimitiveComponent|SetRenderinMainPass _returnvalue true)
    (Rendering|Material|SetMaterial _returnvalue 0 "/Game/Materials/Mat_Color.Mat_Color")))

(fn HideSpatialMeshes
  (params (TrackedGeometry :type AR%20Tracked%20Geometry%20Object%20Reference))
  (bind _returnvalue (Class|ARTrackedGeometry|GetUnderlyingMesh TrackedGeometry))
  (if (Utilities|IsValid _returnvalue)
    (Rendering|SetRenderCustomDepth _returnvalue true)
    (Class|PrimitiveComponent|SetRenderinMainPass _returnvalue false)
    (Rendering|Material|SetMaterial _returnvalue 0 "/Game/Materials/Mat_Occlusion.Mat_Occlusion")))

(fn StartSpatialMapping
  (bind _returnvalue (Class|ARBlueprintLibrary|ToggleARCapture true "SpatialMapping"))
  (if _returnvalue
    (Utilities|Time|SetTimerbyFunctionName 0 "StopSpatialMapping" 6e+01)
    (else
      (Utilities|Time|SetTimerbyFunctionName 0 "StartSpatialMapping" 3.0))))

(fn StopSpatialMapping
  (Class|ARBlueprintLibrary|ToggleARCapture false "SpatialMapping"))